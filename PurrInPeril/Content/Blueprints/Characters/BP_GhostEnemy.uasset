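; Ghost enemy character that emits voice sounds and chases BP_Purr when it sees it.
; A self-rescheduling timer plays the voice at random intervals until the game state reports game over.
; Pawn sensing writes the chase target and sense type to the AI controller's blackboard.
; After a timeout Delay, which repeat sightings do not extend, the sense type reverts if still chasing; the target stays set.
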(event OnSeePawn(PawnSensing)
  (params (Pawn :type Pawn%20Object%20Reference))
  (bind _self self)
  (bind _returnvalue (AI|GetAIController _self))
  (bind _returnvalue_2 (AI|GetBlackboard _returnvalue))
  (bind _asbp_purr (Utilities|Casting|CastToBP_Purr Pawn))
  (AI|Components|Blackboard|SetValueasEnum _returnvalue_2 (Utilities|Name|MakeLiteralName "SenseType") (Utilities|Enum|LiteralenumE_AISenseType "NewEnumerator1"))
  (AI|Components|Blackboard|SetValueasObject _returnvalue_2 (Utilities|Name|MakeLiteralName "ChaseTargetActor") _asbp_purr)
  (Utilities|FlowControl|Delay (Variables|Default|GetChaseTimeOutInSecond))
  (if (Utilities|Enum|Equal(Enum) (Utilities|Enum|ByteToEnumE_AISenseType (Class|BlackboardComponent|GetValueasEnum (AI|GetBlackboard (AI|GetAIController self)) (Utilities|Name|MakeLiteralName "SenseType"))) "NewEnumerator1")
    (AI|Components|Blackboard|SetValueasEnum (AI|GetBlackboard (AI|GetAIController self)) (Utilities|Name|MakeLiteralName "SenseType") (Utilities|Enum|LiteralenumE_AISenseType "NewEnumerator0"))))

(event Custom|EmitVoice
  (bind _voicecomponent (Variables|Default|GetVoiceComponent))
  (bind _aspurr_in_peril_main_game_state (Utilities|Casting|CastToPurrInPerilMainGameState (Game|GetGameState)))
  (if (not (Variables|/Script/PurrInPeril.PurrInPerilMainGameState|GetbIsGameOver _aspurr_in_peril_main_game_state))
    (Class|AudioComponent|SetPaused _voicecomponent false)
    (Audio|Components|Audio|Play _voicecomponent 0.0)
    (Utilities|Time|SetTimerbyEvent (delegate Custom|EmitVoice) (Math|Random|RandomFloatinRange (Variables|Default|GetMinRandomVoiceEmitInSecond) (Variables|Default|GetMaxRandomVoiceEmitInSecond)))))

(event EventBeginPlay
  (Class|AudioComponent|SetPaused (Variables|Default|GetVoiceComponent) true)
  (Utilities|Time|SetTimerbyEvent (delegate Custom|EmitVoice) (Math|Random|RandomFloatinRange (Variables|Default|GetMinRandomVoiceEmitInSecond) (Variables|Default|GetMaxRandomVoiceEmitInSecond))))

(fn ConstructionScript)