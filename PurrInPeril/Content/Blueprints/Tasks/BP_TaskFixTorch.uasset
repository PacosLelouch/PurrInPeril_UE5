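; Task actor for fixing a torch: a spotlight that flickers until its part of the task is completed.
; A self-rescheduling random-interval timer toggles the light's visibility while the first player controller has not completed the part.
; Completion calls the parent logic, then recolors the light and leaves it visible.
; Overlap events defer to the parent and print debug strings.
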(event Custom|FlipLight
  (bind _spotlight (Variables|Default|GetSpotLight))
  (if (not (Class|PurrinPerilTaskActorBase|IsThisPartOfTaskCompleted (Game|GetPlayerController 0)))
    (Rendering|SetVisibility _spotlight (not (Variables|/Script/Engine.SceneComponent|GetbVisible _spotlight)) false)
    (Utilities|Time|SetTimerbyEvent (delegate Custom|FlipLight) (Math|Random|RandomFloatinRange 0.5 1.5))))

(event EventBeginPlay
  (if (not (Class|PurrinPerilTaskActorBase|IsThisPartOfTaskCompleted (Game|GetPlayerController 0)))
    (Utilities|Time|SetTimerbyEvent (delegate Custom|FlipLight) (Math|Random|RandomFloatinRange 0.5 1.5))))

(event EventCompleteThisPartOfTask
  (params (Controller :type Controller%20Object%20Reference))
  (bind _spotlight (Variables|Default|GetSpotLight))
  (|CallParentFunction Controller)
  (Rendering|Components|Light|SetLightColor _spotlight "(R=0.400000,G=0.400000,B=0.300000,A=1.000000)" true)
  (Rendering|SetVisibility _spotlight true false))

(event Collision|EventActorBeginOverlap
  (params (OtherActor :type Actor%20Object%20Reference))
  (|CallParentFunction OtherActor)
  (Development|PrintString "Hello"))

(event Collision|EventActorEndOverlap
  (params (OtherActor :type Actor%20Object%20Reference))
  (|CallParentFunction OtherActor)
  (Development|PrintString "Bye"))

(fn ConstructionScript)