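; BP_FinalTask is the hidden final task of Purr In Peril, which triggers a temporary win when interacted with.
; It starts invisible, scentless and without overlap.
; In the last 40 seconds, Tick compares task totals from the task subsystem and reveals it on a match, though the completed count is overwritten rather than summed.
; Interaction calls WinTemp on the player controller and starts the mesh spinning.
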(event EventBeginPlay
  (Rendering|SetVisibility (Variables|Transformation|GetRootComponent) false true)
  (Variables|/Script/PurrInPeril.PurrInPerilSmellProduceComponent|SetbWithSmell (Variables|Default|GetSmellProduceComponent) false)
  (Variables|/Script/Engine.PrimitiveComponent|SetbGenerateOverlapEvents (Variables|Default|GetInteractableComponent) false))

(event EventCompleteThisPartOfTask
  (params (Controller :type Controller%20Object%20Reference))
  (bind _asbp_purr_in_peril_main_player_controller (Utilities|Casting|CastToBP_PurrInPerilMainPlayerController Controller))
  (Default|WinTemp _asbp_purr_in_peril_main_player_controller)
  (Variables|Default|SetbCompleted true))

(event EventTick
  (params (DeltaSeconds :type Float%20%28single-precision%29))
  (bind _returnvalue (Subsystems|GetPurrinPerilTaskManagementSubsystem))
  (Utilities|FlowControl|Sequence
    (:then_0
      (if (Variables|Default|GetbCompleted)
        (Transformation|AddRelativeRotation (Variables|Default|GetStaticMesh) (Math|Rotator|MakeRotator 0.0 0.0 (* DeltaSeconds 15.0)) false false)))
    (:then_1
      (bind _aspurr_in_peril_main_game_state (Utilities|Casting|CastToPurrInPerilMainGameState (Game|GetGameState)))
      (if (and (not (Variables|Default|GetbAppeared)) (<= (Variables|/Script/PurrInPeril.PurrInPerilMainGameState|GetCurrentCountdownInSecond _aspurr_in_peril_main_game_state) 4e+01))
        (Utilities|FlowControl|Sequence
          (:then_0
            (Variables|Default|SetNumTask 0)
            (Variables|Default|SetNumTaskCompleted 0))
          (:then_1
            (bind _keys (Utilities|Map|Keys (Variables|/Script/PurrInPeril.PurrInPerilTaskManagementSubsystem|GetTaskActors _returnvalue)))
            (for _array_element _keys
              (if (== _array_element (Class|TaskIdentifierMapping|GetIdentifier (Class|PurrinPerilAssetLibrary|GetTaskIdentifierMappingfromGameInstance) (Utilities|GetClass self)))
                (Math|Integer|IncrementInt (Variables|Default|GetNumTaskCompleted))
                (else
                  (Variables|Default|SetNumTask (+ (Variables|Default|GetNumTask) (.TaskNum (Utilities|Struct|BreakPurrInPerilTaskNum (Class|PurrinPerilTaskManagementSubsystem|GetTaskNumandCompleteCount _returnvalue _array_element (Game|GetPlayerController 0))))))
                  (Variables|Default|SetNumTaskCompleted (+ 0 (.TaskCompleteNum (Utilities|Struct|BreakPurrInPerilTaskNum (Class|PurrinPerilTaskManagementSubsystem|GetTaskNumandCompleteCount _returnvalue _array_element (Game|GetPlayerController 0))))))))))
          (:then_2
            (if (== (Variables|Default|GetNumTaskCompleted) (Variables|Default|GetNumTask))
              (Variables|/Script/PurrInPeril.PurrInPerilSmellProduceComponent|SetbWithSmell (Variables|Default|GetSmellProduceComponent) true)
              (Rendering|SetVisibility (Variables|Transformation|GetRootComponent) true true)
              (Variables|/Script/Engine.PrimitiveComponent|SetbGenerateOverlapEvents (Variables|Default|GetInteractableComponent) true)
              (Variables|Default|SetbAppeared true))))))))

(event Collision|EventActorBeginOverlap
  (params (OtherActor :type Actor%20Object%20Reference))
  (|CallParentFunction OtherActor)
  (Development|PrintString "Hello"))

(event Collision|EventActorEndOverlap
  (params (OtherActor :type Actor%20Object%20Reference))
  (|CallParentFunction OtherActor)
  (Development|PrintString "Bye"))

(event EventOpenInteraction
  (params (Controller :type Controller%20Object%20Reference))
  (|CallParentFunction Controller)
  (Class|PurrinPerilTaskActorBase|CompleteThisPartOfTask Controller))

(fn ConstructionScript)