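; AI controller for the main enemy in Purr In Peril, which runs the BT_MonsterAI behavior tree on BeginPlay.
; It reacts to emitted sounds tagged FoodInteraction and to the player completing part of a task.
; Each event writes a sense type and the source's world location to the Blackboard, using separate location keys for sounds and tasks.
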(event EventBeginPlay
  (AI|RunBehaviorTree "/Game/Blueprints/AI/BT_MonsterAI.BT_MonsterAI"))

(event EventTick
  (params (DeltaSeconds :type Float%20%28single-precision%29)))

(event EventOnSoundEmitted
  (params (AudioEmitted :type Purr%20in%20Peril%20Environment%20Audio%20Component%20Object%20Reference))
  (bind _blackboard (Variables|Default|GetBlackboard))
  (if (== (Variables|/Script/PurrInPeril.PurrInPerilEnvironmentAudioComponent|GetAudioTag AudioEmitted) "FoodInteraction")
    (Utilities|FlowControl|Sequence
      (:then_0
        (AI|Components|Blackboard|SetValueasEnum _blackboard (Utilities|Name|MakeLiteralName "SenseType") (Utilities|Enum|LiteralenumE_AISenseType "NewEnumerator2")))
      (:then_1
        (AI|Components|Blackboard|SetValueasVector _blackboard (Utilities|Name|MakeLiteralName "SoundLocation") (Transformation|GetWorldLocation AudioEmitted))))))

(event EventOnPlayerCompletePartOfTask
  (params (TaskActor :type Purr%20in%20Peril%20Task%20Actor%20Base%20Object%20Reference) (Controller :type Controller%20Object%20Reference))
  (bind _blackboard (Variables|Default|GetBlackboard))
  (Utilities|FlowControl|Sequence
    (:then_0
      (AI|Components|Blackboard|SetValueasEnum _blackboard (Utilities|Name|MakeLiteralName "SenseType") (Utilities|Enum|LiteralenumE_AISenseType "NewEnumerator3")))
    (:then_1
      (AI|Components|Blackboard|SetValueasVector _blackboard (Utilities|Name|MakeLiteralName "TaskCompleteLocation") (Transformation|GetWorldLocation (Variables|/Script/Engine.Actor|GetRootComponent TaskActor))))))

(fn ConstructionScript)