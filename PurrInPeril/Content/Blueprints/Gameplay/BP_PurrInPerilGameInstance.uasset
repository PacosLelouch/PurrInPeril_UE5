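; Game instance Blueprint for Purr In Peril that provides toggles for engine performance stat overlays.
; Separate events for Unit, GPU and FPS stats each run the matching stat console command, then flip a boolean that tracks that overlay's state.
; Each boolean is inverted blindly alongside its command rather than read from the engine.
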(event Custom|StatUnit
  (Development|ExecuteConsoleCommand "stat unit" 0)
  (Variables|Default|SetbEnableStatUnit (not (Variables|Default|GetbEnableStatUnit))))

(event Custom|StatGPU
  (Development|ExecuteConsoleCommand "stat gpu" 0)
  (Variables|Default|SetbEnableStatGPU (not (Variables|Default|GetbEnableStatGPU))))

(event Custom|StatFPS
  (Development|ExecuteConsoleCommand "stat fps" 0)
  (Variables|Default|SetbEnableStatFPS (not (Variables|Default|GetbEnableStatFPS))))