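; BP_PurrInPerilMainPlayerState is the main level's player state, which watches for the player's losing conditions.
; Each Tick it checks whether the game state's countdown has run out or the player's Sanity or Hunger equals zero.
; If so, and the game state is not already game over, it calls Lose on the main player controller.
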(event EventBeginPlay)

(event EventTick
  (params (DeltaSeconds :type Float%20%28single-precision%29))
  (bind _currentplayerstateparameter (Variables|Default|GetCurrentPlayerStateParameter))
  (bind (_sanityvalue _hungervalue) (Utilities|Struct|BreakPlayerStateParameter _currentplayerstateparameter))
  (bind _aspurr_in_peril_main_game_state (Utilities|Casting|CastToPurrInPerilMainGameState (Game|GetGameState)))
  (if (or (<= (Variables|/Script/PurrInPeril.PurrInPerilMainGameState|GetCurrentCountdownInSecond _aspurr_in_peril_main_game_state) 0.0) (or (== _sanityvalue 0.0) (== _hungervalue 0.0)))
    (if (not (Variables|/Script/PurrInPeril.PurrInPerilMainGameState|GetbIsGameOver _aspurr_in_peril_main_game_state))
      (bind _asbp_purr_in_peril_main_player_controller (Utilities|Casting|CastToBP_PurrInPerilMainPlayerController (Game|GetPlayerController)))
      (Default|Lose _asbp_purr_in_peril_main_player_controller false))))

(fn ConstructionScript)