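; Cat food Blueprint that responds when the player interacts with it in Purr In Peril.
; It extends the parent food interaction event, playing the BP_Purr pawn's eat sound on success.
; It then creates a top message widget, with text built from food name, cooldown, durability and success, and adds it to the player's foreground panel.
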(event EventBeginPlay)

(event Collision|EventActorBeginOverlap
  (params (OtherActor :type Actor%20Object%20Reference)))

(event EventTick
  (params (DeltaSeconds :type Float%20%28single-precision%29)))

(event EventOnFoodInteractwithPlayer
  (params (Controller :type Controller%20Object%20Reference) (bSucceeded :type Boolean))
  (|CallParentFunction Controller bSucceeded)
  (Utilities|FlowControl|Sequence
    (:then_0
      (if bSucceeded
        (bind _asbp_purr (Utilities|Casting|CastToBP_Purr (Pawn|GetControlledPawn Controller)))
        (Default|EatSound _asbp_purr)))
    (:then_1
      (bind _aspurr_in_peril_main_player_controller (Utilities|Casting|CastToPurrInPerilMainPlayerController Controller))
      (bind _returnvalue (UserInterface|CreateWidget "/Game/Blueprints/Widgets/Messages/BPW_TopMessageWidget.BPW_TopMessageWidget_C" _aspurr_in_peril_main_player_controller))
      (Rendering|Components|TextRender|SetText (Variables|/Game/Blueprints/Widgets/Messages/BPW_TopMessageWidget.BPW_TopMessageWidget_C|GetText_MultiLineMessage _returnvalue) (CallFunction|GetFoodTopMessage "Cat Food" (Variables|Default|GetCurrentInteractColdDownInSecond) bSucceeded (Variables|Default|GetDurability)))
      (bind _asbpw_player_main_foreground_panel_widget (Utilities|Casting|CastToBPW_PlayerMainForegroundPanelWidget (Variables|/Script/PurrInPeril.PurrInPerilMainPlayerController|GetPlayerMainForegroundPanelWidget _aspurr_in_peril_main_player_controller)))
      (Widget|Panel|AddChild (Variables|/Game/Blueprints/Widgets/BPW_PlayerMainForegroundPanelWidget.BPW_PlayerMainForegroundPanelWidget_C|GetSlot_TopMessage _asbpw_player_main_foreground_panel_widget) _returnvalue))))

(fn ConstructionScript)