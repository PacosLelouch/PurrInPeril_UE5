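; Blueprint function library that builds the top-of-screen message shown when the player tries to use a food item.
; GetFoodTopMessage branches on success and remaining durability to report the food as used up, used with a cooldown, or still cooling down.
; Each message is built with FormatText from the food name and the cooldown floored to whole seconds.
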(fn GetFoodTopMessage
  (params (FoodName :type Text) (ColdDownInSecond :type Float%20%28double-precision%29) (bSucceeded :type Boolean) (Durability :type Integer))
  (bind _returnvalue (Class|KismetMathLibrary|FFloor64 ColdDownInSecond))
  (if bSucceeded
    (if (== Durability 0)
      (return (Utilities|Text|FormatText (Utilities|Text|MakeLiteralText "\"{FoodName}\" is used. 
It is no longer available!") FoodName))
      (else
        (return (Utilities|Text|FormatText (Utilities|Text|MakeLiteralText "\"{FoodName}\" is used. 
Please wait for {ColdDown} to use for the next time.") FoodName _returnvalue))))
    (else
      (return (Utilities|Text|FormatText (Utilities|Text|MakeLiteralText "Please wait for {ColdDown} second(s) to use it!") _returnvalue)))))